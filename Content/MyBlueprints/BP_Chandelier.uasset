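; BP_Chandelier is a chandelier actor with an animated light that flickers, sways and shifts color from BeginPlay.
; A flicker timeline drives light intensity and plays the sway timeline on each update, which in turn plays a color timeline that sets RGB.
; The sway step offsets the light's owning actor along X, then immediately sets that actor's location to the world origin.
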(event Custom|Sway%20Light
  (bind _newtrack_0 (Timeline|LightSwayMovement Play)
    (:Update
      (Transformation|AddActorLocalOffset (Components|GetOwner (Variables|Default|GetChandelier%20Light)) (Math|Vector|MakeVector _newtrack_0 0.0 0.0) false false)
      (Transformation|SetActorLocation (Components|GetOwner (Variables|Default|GetChandelier%20Light)) "0, 0, 0" false false)
      (Variables|Default|SetChandelier%20Light (Variables|Default|GetChandelier%20Light))
      (CallFunction|SwayColor))))

(event Custom|Sway%20Color
  (bind (_direction _red _green _blue) (Timeline|LightColorSway Play)
    (:Update
      (Rendering|Components|Light|SetLightColor (Variables|Default|GetChandelier%20Light) (Math|Color|MakeColor _red _green _blue) true)
      (Variables|Default|SetChandelier%20Light (Variables|Default|GetChandelier%20Light)))))

(event EventBeginPlay
  (bind _newtrack_0 (Timeline|LightFlicker Play)
    (:Update
      (Rendering|Components|Light|SetIntensity (Variables|Default|GetChandelier%20Light) _newtrack_0)
      (Variables|Default|SetChandelier%20Light (Variables|Default|GetChandelier%20Light))
      (CallFunction|SwayLight))))

(fn ConstructionScript)