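; BP_GiantDoors is a pair of giant Level_One doors that creak open when something overlaps the Open_Trigger collision box, intended for the player.
; A timeline drives the yaw of both doors in opposite directions.
; Each update calls ExecuteDoorSound, where a DoOnce limits the eerie sound to one play, located through GetActorOfClass rather than the actor's own reference.
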(event OnComponentBeginOverlap(Open_Trigger)
  (params (OverlappedComponent :type Primitive%20Component%20Object%20Reference) (OtherActor :type Actor%20Object%20Reference) (OtherComp :type Primitive%20Component%20Object%20Reference) (OtherBodyIndex :type Integer) (bFromSweep :type Boolean) (SweepResult :type Hit%20Result%20Structure%20%28by%20ref%29))
  ;[1 1 1] Animation and Sound for opening Level_One doors
  ;;[0.05098 0.05098 0.05098] Pivots Doors once player enters collision box
  (bind _doorrotation (Timeline|OpenDoorsTimeline Play)
    (:Update
      (Utilities|FlowControl|Sequence
        (:then_0
          (Transformation|SetRelativeRotation (Variables|Default|GetRight_Door) (Math|Rotator|MakeRotator 0.0 0.0 (* -1.0 _doorrotation)) false false)
          (Variables|Default|SetRight_Door (Variables|Default|GetRight_Door)))
        (:then_1
          (Transformation|SetRelativeRotation (Variables|Default|GetLeft_Door) (Math|Rotator|MakeRotator 0.0 0.0 _doorrotation) false false)
          (Variables|Default|SetLeft_Door (Variables|Default|GetLeft_Door))))
      (CallFunction|ExecuteDoorSound))))

(event Custom|Execute%20Door%20Sound
  ;[1 1 1] Animation and Sound for opening Level_One doors
  ;;[0.05098 0.05098 0.05098] Plays creaky door sound while doors open
  (Utilities|FlowControl|DoOnce false
    (:Completed
      (bind _returnvalue (Actor|GetActorOfClass "BP_GiantDoors_C"))
      (Audio|PlaySoundatLocation "/Game/MyAudios/Eerie_Door_B-u_ryiem47seu_.Eerie_Door_B-u_ryiem47seu_" (Transformation|GetActorLocation _returnvalue) "0, 0, 0" 1.0 1.0 0.0 0 0 0 0))))

(fn ConstructionScript)